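; Player character Blueprint for a first-person or third-person shooter, handling crouch and automatic rifle fire.
; Crouch input also sets the AnimBP flag; while left mouse is held, Tick runs a Delay-throttled camera line trace with random recoil, montage, sound and muzzle flash.
; Hits spawn decals and blood or asphalt particles, and call RifleHit on Enemy after the delay.
; Velocity-based spread is clamped to zero; sniper zoom/UI logic is unconnected.
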(event EventBeginPlay)

(event Collision|EventActorBeginOverlap
  (params (OtherActor :type Actor%20Object%20Reference)))

(event EventTick
  (params (DeltaSeconds :type Float%20%28single-precision%29))
  (bind _returnvalue (Transformation|GetVelocity))
  (bind _riflecomp (Variables|Default|GetrifleComp))
  (bind _cameracomp (Variables|Default|GetcameraComp))
  (bind _returnvalue_2 (Math|Vector|ClampVectorSize _returnvalue 0.0 0.0))
  (bind _returnvalue_3 (Transformation|GetSocketTransform _riflecomp "RifleFirePosition" "RTS_World"))
  (bind _returnvalue_4 (Transformation|GetWorldLocation _cameracomp))
  (bind _returnvalue_5 (Math|Vector|VectorLength _returnvalue_2))
  (if (not (Variables|Default|GetbUsingSniper))
    (if (and (Variables|Default|GetcanShoot) (Variables|Default|GetisLMB))
      (bind (_outhit _returnvalue_6) (Collision|LineTraceForObjects _returnvalue_4 (+ _returnvalue_4 (* (Math|Vector|GetForwardVector _cameracomp) 9999.0) (Math|Vector|MakeVector (* _returnvalue_5 (Math|Random|RandomFloatinRange -5e+02 5e+02)) (* _returnvalue_5 (Math|Random|RandomFloatinRange -5e+02 5e+02)) (* _returnvalue_5 (Math|Random|RandomFloatinRange -5e+02 5e+02)))) (Utilities|Array|MakeArray "ObjectTypeQuery1" "ObjectTypeQuery2" "ObjectTypeQuery3" "ObjectTypeQuery4") false 0 "None"))
      (if _returnvalue_6
        (Pawn|Input|AddControllerPitchInput (Math|Random|RandomFloatinRange -0.1 -0.8))
        (Pawn|Input|AddControllerYawInput (Math|Random|RandomFloatinRange -0.4 0.4))
        (else
          (Pawn|Input|AddControllerPitchInput (Math|Random|RandomFloatinRange -0.1 -0.8))
          (Pawn|Input|AddControllerYawInput (Math|Random|RandomFloatinRange -0.4 0.4))))
      (Audio|SpawnSoundatLocation 0 (.location _returnvalue_3) "0, 0, 0" 1.0 1.0 0.0 0 0)
      (Animation|PlayAnimMontage "/Game/MyAnimation/Fire_Rifle_Ironsights_Montage.Fire_Rifle_Ironsights_Montage" 1.0 "None")
      (Effects|SpawnEmitteratLocation "/Game/MyBlueprint/gunfire.gunfire" (.location _returnvalue_3) (.rotation _returnvalue_3) (* (.scale _returnvalue_3) 0.8))
      (Utilities|Casting|CastToBP_Enemy (.HitActor (Collision|BreakHitResult _outhit))
        (:then
          (Game|SpawnActorfromClass "/Game/MyBlueprint/BP_ShotDecal.BP_ShotDecal_C" (Math|Transform|MakeTransform (.Location (Collision|BreakHitResult _outhit)) (Math|Conversions|RotationFromXVector (.ImpactNormal (Collision|BreakHitResult _outhit)))) "Undefined" 0 0)
          (Effects|SpawnEmitteratLocation "/Game/MyBlueprint/BloodParticle.BloodParticle" (.location (Math|Transform|MakeTransform (.Location (Collision|BreakHitResult _outhit)) (Math|Conversions|RotationFromXVector (.ImpactNormal (Collision|BreakHitResult _outhit))))) (.rotation (Math|Transform|MakeTransform (.Location (Collision|BreakHitResult _outhit)) (Math|Conversions|RotationFromXVector (.ImpactNormal (Collision|BreakHitResult _outhit)))))))
        (:CastFailed
          (Game|SpawnActorfromClass "/Game/MyBlueprint/BP_ShotDecal.BP_ShotDecal_C" (Math|Transform|MakeTransform (.Location (Collision|BreakHitResult _outhit)) (Math|Conversions|RotationFromXVector (.ImpactNormal (Collision|BreakHitResult _outhit)))) "Undefined" 0 0)
          (Effects|SpawnEmitteratLocation "/Game/MyBlueprint/P_Asphalt.P_Asphalt" (.location (Math|Transform|MakeTransform (.Location (Collision|BreakHitResult _outhit)) (Math|Conversions|RotationFromXVector (.ImpactNormal (Collision|BreakHitResult _outhit))))) (.rotation (Math|Transform|MakeTransform (.Location (Collision|BreakHitResult _outhit)) (Math|Conversions|RotationFromXVector (.ImpactNormal (Collision|BreakHitResult _outhit))))) "2.500000,2.500000,2.500000")))
      (Variables|Default|SetcanShoot false)
      (Utilities|FlowControl|Delay (/ 1.0 (Variables|Default|GetBullets/sec)))
      (Variables|Default|SetcanShoot true)
      (bind _asenemy (Utilities|Casting|CastToEnemy (.HitActor (Collision|BreakHitResult _outhit))))
      (Class|Enemy|RifleHit _asenemy))))

(event Input|ActionEvents|InputActionCrouch
  (params (Key :type Key%20Structure :default "None"))
  (:Pressed
    (Character|Crouch)
    (bind _asabp_player_character (Utilities|Casting|CastToABP_PlayerCharacter (Components|SkeletalMesh|GetAnimInstance (Variables|Character|GetMesh))))
    (Variables|/Game/MyBlueprint/ABP_PlayerCharacter.ABP_PlayerCharacter_C|SetisCrouch _asabp_player_character true))
  (:Released
    (Character|UnCrouch)
    (bind _asabp_player_character_2 (Utilities|Casting|CastToABP_PlayerCharacter (Components|SkeletalMesh|GetAnimInstance (Variables|Character|GetMesh))))
    (Variables|/Game/MyBlueprint/ABP_PlayerCharacter.ABP_PlayerCharacter_C|SetisCrouch _asabp_player_character_2 false)))

(event Input|ActionEvents|InputActionZoom
  (params (Key :type Key%20Structure :default "None")))

(event Input|MouseEvents|LeftMouseButton
  (params (Key :type Key%20Structure :default "None"))
  (:Pressed
    (Variables|Default|SetisLMB true))
  (:Released
    (Variables|Default|SetisLMB false)))

(fn ConstructionScript)